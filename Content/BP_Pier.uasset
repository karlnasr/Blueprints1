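; BP_Pier is a procedural wooden-style pier actor built entirely in the construction script, with no runtime logic.
; A loop over StepsCount adds flattened static mesh planks at even spacing along Y, each with a slight random roll, pitch and yaw for a hand-built look.
; Every fourth step also adds a pair of upright post meshes, one on each side.
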(event EventBeginPlay)

(event Collision|EventActorBeginOverlap
  (params (OtherActor :type Actor%20Object%20Reference)))

(event EventTick
  (params (DeltaSeconds :type Float%20%28single-precision%29)))

(fn ConstructionScript
  (for _index (range 0 (+ (Variables|Default|GetSteps%20Count) 0))
    (AddComponent|AddStaticMeshComponent false (Math|Transform|MakeTransform (Math|Vector|MakeVector 0.0 (Math|Conversions|ToFloat(Integer) (* _index 32)) 8e+01) (Math|Rotator|MakeRotator (Math|Random|RandomFloatinRange -3.0 3.0) (Math|Random|RandomFloatinRange -1.0 1.0) (Math|Random|RandomFloatinRange -2.0 2.0)) "1,0.300000,0.030000"))
    (if (== (Math|Integer|%(Integer) _index 4) 0)
      (AddComponent|AddStaticMeshComponent false (Math|Transform|MakeTransform (Math|Vector|MakeVector 6e+01 (Math|Conversions|ToFloat(Integer) (* _index 32)) 5e+01) "0, 0, 0" "0.200000,0.200000,1"))
      (AddComponent|AddStaticMeshComponent false (Math|Transform|MakeTransform (Math|Vector|MakeVector -6e+01 (Math|Conversions|ToFloat(Integer) (* _index 32)) 5e+01) "0, 0, 0" "0.200000,0.200000,1")))))