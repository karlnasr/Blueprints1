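; BP_Button is an overlap-triggered button actor that shows its pressed state by color.
; Begin and end overlap call the ButtonPressed and ButtonReleased events, with no filter on the overlapping actor.
; Pressing creates a new dynamic material instance from M_Basic_Red on Cylinder1 and sets its Color parameter to green.
; Releasing sets the stored instance back to red.
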(event Custom|Button%20Released
  (Rendering|Material|SetVectorParameterValue (Variables|Default|GetButtonMaterial) "Color" "(R=0.741667,G=0.020979,B=0.000000,A=1.000000)" :!class /Script/Engine.MaterialInstanceDynamic))

(event Custom|Button%20Pressed
  (bind _returnvalue (Rendering|Material|CreateDynamicMaterialInstance (Variables|Default|GetCylinder1) 0 "/Game/M_Basic_Red.M_Basic_Red" "None" :!class /Script/Engine.PrimitiveComponent))
  (bind _output_get (Variables|Default|SetButtonMaterial _returnvalue))
  (Rendering|Material|SetVectorParameterValue _output_get "Color" "(R=0.095575,G=0.758333,B=0.000000,A=1.000000)" :!class /Script/Engine.MaterialInstanceDynamic))

(event Collision|EventActorBeginOverlap
  (params (OtherActor :type Actor%20Object%20Reference))
  (CallFunction|ButtonPressed))

(event Collision|EventActorEndOverlap
  (params (OtherActor :type Actor%20Object%20Reference))
  (CallFunction|ButtonReleased))

(fn ConstructionScript)