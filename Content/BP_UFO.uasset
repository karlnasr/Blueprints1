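; Actor Blueprint for a UFO that hovers at a set height above the surface beneath it.
; On BeginPlay, a short downward line trace snaps the actor to that height above the hit point.
; The UFOAnimation timeline's update lerps the SUFO component's relative location and rotation to bob, tilt and spin it, though no exec wire starts the timeline here.
; The construction script sets its play rate from Speed.
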(event EventBeginPlay
  (CallFunction|UpdateHeight 1.5e+02))

(fn ConstructionScript
  (Components|Timeline|SetPlayRate (Variables|Default|GetUFOAnimation) (Variables|Default|GetSpeed)))

(fn UpdateHeight
  (params (DesiredHeight :type Float%20%28single-precision%29))
  (bind _returnvalue (Transformation|GetActorLocation))
  (bind (_outhit _returnvalue_2) (Collision|LineTraceByChannel _returnvalue (- _returnvalue "0, 0,300.000000") "TraceTypeQuery1" false 0 "None"))
  (if _returnvalue_2
    (if (!= (Math|Vector|Distance(Vector) (Transformation|GetActorLocation) (.Location (Collision|BreakHitResult _outhit))) DesiredHeight)
      (Transformation|SetActorLocation (+ (.Location (Collision|BreakHitResult _outhit)) (Math|Vector|MakeVector 0.0 0.0 DesiredHeight)) false false))))